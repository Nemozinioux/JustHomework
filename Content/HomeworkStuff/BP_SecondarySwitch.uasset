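; BP_SecondarySwitch is an interactable switch that stays locked until a linked main switch is triggered, then rotates a set of doors.
; On BeginPlay it binds Unlock to the main switch's OnMainButtonTriggered dispatcher; Unlock marks it available and changes the switch material.
; Interact calls Rotate on each door in DoorsToRotate when available, and prints a click or locked message.
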(event Custom|Unlock
  (Variables|Default|SetIsSwitchAvailable true)
  (Rendering|Material|SetMaterial (Variables|Default|GetSwitch) 0 "/Engine/BasicShapes/BasicShapeMaterial.BasicShapeMaterial"))

(event EventBeginPlay
  (EventDispatchers|BindEventtoOnMainButtonTriggered (Variables|Default|GetMainSwitch) (delegate Custom|Unlock)))

(event EventInteract
  (if (Variables|Default|GetIsSwitchAvailable)
    (Development|PrintString "Click")
    (for _array_element (Variables|Default|GetDoorsToRotate)
      (Default|Rotate _array_element))
    (else
      (Development|PrintString "Switch is locked"))))

(fn ConstructionScript)